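; Game instance Blueprint that holds persistent player settings and an audio playback helper.
; Play Audio creates a 2D sound with a given volume and optional persistence across level transitions, stores it in Audio and plays it.
; Separate Make functions set default values for mouse sensitivity, master, music and effects volumes, and brightness.
; GetPostProcces only clears the stored post-process settings reference.
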(fn PlayAudio
  (params (Sound :type Sound%20Base%20Object%20Reference) (Volume :type Float%20%28single-precision%29) (Persist? :type Boolean))
  (bind _returnvalue (Audio|CreateSound2D Sound Volume 1.0 0.0 0 Persist?))
  (bind _output_get (Variables|Default|SetAudio _returnvalue))
  (Audio|Components|Audio|Play _output_get 0.0))

(fn MakeMouseSens
  (Variables|Default|SetMouseSens 45.0))

(fn MakeVolume
  (Variables|Default|SetMasterVolume 1.0)
  (Variables|Default|SetMusicVol 1.0)
  (Variables|Default|SetFXVol 1.0))

(fn MakeBrightness
  (Variables|Default|SetBrightness 0.0))

(fn GetPostProcces
  (Variables|Default|SetPostProccesSettings ""))