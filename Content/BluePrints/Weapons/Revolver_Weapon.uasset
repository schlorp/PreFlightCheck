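; Revolver weapon for the player character, with six rounds, random bullet spread, timed reload and ammo state saved to the SecondaryWeapon slot on unequip.
; Fire decrements ammo, runs debug-drawn traces from camera then muzzle, spawns a decal and occasional tracer, then plays an ADS-dependent montage and muzzle flash.
; An empty gun plays a sound instead.
; Reload is DoOnce-gated and refills ammo after a delay.
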(event EventFire
  (bind _returnvalue (Game|GetPlayerCharacter 0))
  (bind _asbp_player_character (Utilities|Casting|CastToBp_PlayerCharacter _returnvalue))
  (bind _mesh (Variables|/Script/Engine.Character|GetMesh _asbp_player_character))
  (if (> (Variables|Default|GetAmmoCount) 0)
    (CallFunction|AmmoCheck)
    (bind (_muzzleloc _impactpoint) (CallFunction|LineTrace))
    (CallFunction|SpawnDecalTracer _muzzleloc _impactpoint _impactpoint)
    (if (Variables|/Game/Models/Bp_PlayerCharacter.Bp_PlayerCharacter_C|GetADS _asbp_player_character)
      (Animation|Montage|PlayMontage _mesh 0
        (:then
          _))
      (else
        (Animation|Montage|PlayMontage _mesh "/Game/_Main/Models/Char/Anim/fps_fire_montage.fps_fire_montage"
          (:then
            _))))
    (Utilities|MuzzleFlash)
    (else
      (Audio|PlaySoundatLocation 0 (Transformation|GetWorldLocation (Variables|/Game/Models/Bp_PlayerCharacter.Bp_PlayerCharacter_C|GetCameraComp (.AsBp%20Player%20Character (Utilities|Casting|CastToBp_PlayerCharacter (Game|GetPlayerCharacter 0))))) "0, 0, 0" 1.0 1.0 0.0 0 0 0 0))))

(event EventReload
  (bind _returnvalue (Game|GetPlayerCharacter 0))
  (bind _asbp_player_character (Utilities|Casting|CastToBp_PlayerCharacter _returnvalue))
  (if (< (Variables|Default|GetAmmoCount) (Variables|Default|GetMaxAmmo))
    (Utilities|FlowControl|DoOnce false :!label _label
      (:Completed
        (Variables|/Game/Models/Bp_PlayerCharacter.Bp_PlayerCharacter_C|SetisReloading _asbp_player_character true)
        (Animation|Montage|MontagePlay (Components|SkeletalMesh|GetAnimInstance (Variables|/Script/Engine.Character|GetMesh _asbp_player_character)) 0 1.0 "MontageLength" 0.0 true)
        (Components|Animation|PlayAnimation (Variables|Default|GetPrimaryWeapon) "/Game/_Main/Models/MilitaryWeapSilver/Weapons/Animations/Reload_SniperRifle_Hip_W.Reload_SniperRifle_Hip_W" false)
        (Utilities|FlowControl|Delay (Variables|Default|GetReloadTime))
        (Variables|Default|SetAmmoCount (Variables|Default|GetMaxAmmo))
        (Variables|/Game/Models/Bp_PlayerCharacter.Bp_PlayerCharacter_C|SetisReloading _asbp_player_character false)
        (goto _label Reset)))))

(event EventUnequip
  (Variables|/Game/Models/Bp_PlayerCharacter.Bp_PlayerCharacter_C|SetSecondaryWeapon (.AsBp%20Player%20Character (Utilities|Casting|CastToBp_PlayerCharacter (Game|GetPlayerCharacter 0))) (Utilities|Struct|MakeGunData "NewEnumerator3" "Revolver_Weapon_C" (Variables|Default|GetAmmoCount) (Variables|Default|GetMaxAmmo) (Variables|Default|GetReloadTime) (Variables|Default|GetBulletSpread))))

(fn ConstructionScript
  (|CallParentFunction)
  (Variables|Default|SetMaxAmmo 6)
  (Variables|Default|SetAmmoCount 6)
  (Variables|Default|SetReloadTime 3.0)
  (Variables|Default|SetBulletSpread 5e+02)
  (Variables|Default|SetName "NewEnumerator3"))

(fn AmmoCheck
  (bind _returnvalue (Math|Random|RandomFloatinRange 7.0 12.0))
  (Math|Integer|DecrementInt (Variables|Default|GetAmmoCount)
    (:%20%20
      (if (Variables|/Game/Models/Bp_PlayerCharacter.Bp_PlayerCharacter_C|GetisReloading (.AsBp%20Player%20Character (Utilities|Casting|CastToBp_PlayerCharacter (Game|GetPlayerCharacter 0))))
        (Audio|PlaySoundatLocation 0 (Transformation|GetWorldLocation (Variables|/Game/Models/Bp_PlayerCharacter.Bp_PlayerCharacter_C|GetCameraComp (.AsBp%20Player%20Character (Utilities|Casting|CastToBp_PlayerCharacter (Game|GetPlayerCharacter 0))))) "0, 0, 0" (+ _returnvalue 2.5) _returnvalue 0.0 0 0 0 0)
        (Components|Animation|PlayAnimation (Variables|Default|GetPrimaryWeapon) "/Game/_Main/Animations/RevolverFire.RevolverFire" false)))))

(fn LineTrace
  (bind _returnvalue (Game|GetPlayerCharacter 0))
  (bind _bulletspread (Variables|Default|GetBulletSpread))
  (bind _asbp_player_character (Utilities|Casting|CastToBp_PlayerCharacter _returnvalue))
  (bind _returnvalue_2 (* _bulletspread -1.0))
  (bind _cameracomp (Variables|/Game/Models/Bp_PlayerCharacter.Bp_PlayerCharacter_C|GetCameraComp _asbp_player_character))
  (bind _returnvalue_3 (Transformation|GetWorldLocation _cameracomp))
  (bind _outhit (Collision|LineTraceByChannel _returnvalue_3 (+ (+ _returnvalue_3 (* (Math|Vector|GetForwardVector _cameracomp) 2e+04)) (Math|Vector|MakeVector (Math|Random|RandomFloatinRange _returnvalue_2 _bulletspread) (Math|Random|RandomFloatinRange _returnvalue_2 _bulletspread) (Math|Random|RandomFloatinRange _returnvalue_2 _bulletspread))) "TraceTypeQuery1" false 0 "ForDuration")) ; Camera Shot
  (Collision|LineTraceByChannel (Transformation|GetWorldLocation (Variables|Default|GetMuzzle)) (.ImpactPoint (Collision|BreakHitResult _outhit)) "TraceTypeQuery1" false 0 "ForDuration" true "(R=0.000000,G=1.000000,B=0.000000,A=1.000000)") ; Gun  Shot
)

(fn SpawnDecalTracer
  (params (Location :type Vector) (SpawnTransform :type Vector) (ImpactPoint :type Vector))
  (Game|SpawnActorfromClass "/Game/_Main/BluePrints/HUD/BulletDecal_BP.BulletDecal_BP_C" (Math|Transform|MakeTransform SpawnTransform (Math|Conversions|RotationFromXVector ImpactPoint) "0.025000,0.025000,0.025000") "Undefined" 0 0)
  (if (>= (Math|Random|RandomIntegerinRange 1 10) 7)
    (Game|SpawnActorfromClass "/Game/_Main/BluePrints/Weapons/TracerRounds_BP.TracerRounds_BP_C" (Math|Transform|MakeTransform Location (Transformation|GetWorldRotation (Variables|/Game/Models/Bp_PlayerCharacter.Bp_PlayerCharacter_C|GetCameraComp (.AsBp%20Player%20Character (Utilities|Casting|CastToBp_PlayerCharacter (Game|GetPlayerCharacter 0))))) "0.100000,0.100000,0.100000") "Undefined" 0 0))
  (return))