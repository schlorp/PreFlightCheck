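; Assault rifle weapon Blueprint for the player, handling firing, timed reloads and saving its stats to the player on unequip.
; Fire makes noise, spends ammo, then uses a spread-randomised camera trace to aim a second trace from the muzzle that applies damage.
; It also spawns bullet decals and occasional tracers, plays hip or ADS montages and flashes a randomised muzzle light and plane; an empty magazine dry-fires.
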(event EventFire
  (bind _returnvalue (Game|GetPlayerCharacter 0))
  (bind _returnvalue_2 (Game|GetPlayerCharacter 0))
  (bind _asbp_player_character (Utilities|Casting|CastToBp_PlayerCharacter _returnvalue))
  (bind _asbp_player_character_2 (Utilities|Casting|CastToBp_PlayerCharacter _returnvalue_2))
  (bind _cameracomp (Variables|/Game/Bp_PlayerCharacter.Bp_PlayerCharacter_C|GetCameraComp _asbp_player_character))
  (bind _returnvalue_3 (Transformation|GetWorldLocation _cameracomp))
  (Class|Actor|MakeNoise (Variables|Default|Getplayer%20character) (Variables|Default|GetLoudness) 0 _returnvalue_3 (Variables|Default|GetNoise%20Range) "None")
  (if (> (Variables|Default|GetAmmoCount) 0)
    (CallFunction|AmmoCheck)
    (Variables|Default|SetLastShotTime (Utilities|Time|GetGameTimeinSeconds))
    (bind (_muzzleloc _impactpoint) (CallFunction|LineTrace))
    (CallFunction|SpawnDecalTracer _muzzleloc _impactpoint _impactpoint)
    (if (Variables|/Game/Bp_PlayerCharacter.Bp_PlayerCharacter_C|GetADS _asbp_player_character_2)
      (Animation|Montage|PlayMontage (Variables|/Script/Engine.Character|GetMesh _asbp_player_character_2) 0
        (:then
          _))
      (else
        (Animation|Montage|PlayMontage 0 "/Game/_Main/Models/Char/Anim/fps_fire_montage.fps_fire_montage"
          (:then
            _))))
    (Utilities|MuzzleFlash)
    (else
      (Audio|PlaySoundatLocation "/Game/_Main/Models/Springfield/DryFire.DryFire" _returnvalue_3 "0, 0, 0" 1.0 1.0 0.0 "/Game/_Main/Models/Springfield/SF_att.SF_att" "/Game/_Main/Models/Springfield/SF_Concurrency.SF_Concurrency" 0 0))))

(event EventUnequip
  (Variables|/Game/Bp_PlayerCharacter.Bp_PlayerCharacter_C|SetPrimaryWeapon (.AsBp%20Player%20Character (Utilities|Casting|CastToBp_PlayerCharacter (Game|GetPlayerCharacter 0))) (Utilities|Struct|MakeGunData "NewEnumerator2" "AR_Weapon_C" (Variables|Default|GetAmmoCount) (Variables|Default|GetMaxAmmo) (Variables|Default|GetReloadTime) (Variables|Default|GetBulletSpread))))

(event EventReload
  (bind _returnvalue (Game|GetPlayerCharacter 0))
  (bind _asbp_player_character (Utilities|Casting|CastToBp_PlayerCharacter _returnvalue))
  (if (< (Variables|Default|GetAmmoCount) (Variables|Default|GetMaxAmmo))
    (Utilities|FlowControl|DoOnce false :!label _label
      (:Completed
        (Variables|/Game/Bp_PlayerCharacter.Bp_PlayerCharacter_C|SetisReloading _asbp_player_character true)
        (Animation|Montage|MontagePlay (Components|SkeletalMesh|GetAnimInstance (Variables|/Script/Engine.Character|GetMesh _asbp_player_character)) "/Game/_Main/Models/AR/Assault_Rifle_A_Skeleton_Montage.Assault_Rifle_A_Skeleton_Montage" 1.0 "MontageLength" 0.0 true)
        (Components|Animation|PlayAnimation (Variables|Default|GetPrimaryWeapon) "/Game/AnimStarterPack/Reload_Rifle_Hip.Reload_Rifle_Hip" false)
        (Utilities|FlowControl|Delay (Variables|Default|GetReloadTime))
        (Variables|Default|SetAmmoCount (Variables|Default|GetMaxAmmo))
        (Variables|/Game/Bp_PlayerCharacter.Bp_PlayerCharacter_C|SetisReloading _asbp_player_character false)
        (goto _label Reset)))))

(fn ConstructionScript
  (|CallParentFunction)
  (Variables|Default|SetMaxAmmo 30)
  (Variables|Default|SetAmmoCount 30)
  (Variables|Default|SetReloadTime 1.7)
  (Variables|Default|SetBulletSpread 5e+02)
  (Variables|Default|SetName "NewEnumerator2"))

(fn AmmoCheck
  (bind _returnvalue (Math|Random|RandomFloatinRange 0.7 1.2))
  (Math|Integer|DecrementInt (Variables|Default|GetAmmoCount)
    (:%20%20
      (if (Variables|/Game/Bp_PlayerCharacter.Bp_PlayerCharacter_C|GetisReloading (.AsBp%20Player%20Character (Utilities|Casting|CastToBp_PlayerCharacter (Game|GetPlayerCharacter 0))))
        (Audio|PlaySoundatLocation "/Game/_Main/Models/Springfield/Gunshot.Gunshot" (Transformation|GetWorldLocation (Variables|/Game/Bp_PlayerCharacter.Bp_PlayerCharacter_C|GetCameraComp (.AsBp%20Player%20Character (Utilities|Casting|CastToBp_PlayerCharacter (Game|GetPlayerCharacter 0))))) "0, 0, 0" (+ _returnvalue 2.5) _returnvalue 0.0 "/Game/_Main/Models/Springfield/SF_att.SF_att" "/Game/_Main/Models/Springfield/SF_Concurrency.SF_Concurrency" 0 0)
        (Components|Animation|PlayAnimation (Variables|Default|GetPrimaryWeapon) "/Game/AnimStarterPack/Fire_Rifle_Hip.Fire_Rifle_Hip" false)))))

(fn LineTrace
  (bind _returnvalue (Game|GetPlayerCharacter 0))
  (bind _bulletspread (Variables|Default|GetBulletSpread))
  (bind _asbp_player_character (Utilities|Casting|CastToBp_PlayerCharacter _returnvalue))
  (bind _returnvalue_2 (* _bulletspread -1.0))
  (bind _cameracomp (Variables|/Game/Bp_PlayerCharacter.Bp_PlayerCharacter_C|GetCameraComp _asbp_player_character))
  (bind _returnvalue_3 (Transformation|GetWorldLocation _cameracomp))
  (bind _outhit (Collision|LineTraceByChannel _returnvalue_3 (+ (+ _returnvalue_3 (* (Math|Vector|GetForwardVector _cameracomp) 2e+04)) (Math|Vector|MakeVector (Math|Random|RandomFloatinRange _returnvalue_2 _bulletspread) (Math|Random|RandomFloatinRange _returnvalue_2 _bulletspread) (Math|Random|RandomFloatinRange _returnvalue_2 _bulletspread))) "TraceTypeQuery1" false 0 "ForDuration")) ; Camera Shot
  (bind _outhit_2 (Collision|LineTraceByChannel (Transformation|GetWorldLocation (Variables|Default|GetMuzzle)) (.ImpactPoint (Collision|BreakHitResult _outhit)) "TraceTypeQuery1" false 0 "ForDuration" true "(R=0.000000,G=1.000000,B=0.000000,A=1.000000)")) ; Gun  Shot
  (Game|Damage|ApplyDamage (.HitActor (Collision|BreakHitResult _outhit_2)) 5e+01 0 0))

(fn SpawnDecalTracer
  (params (Location :type Vector) (SpawnTransform :type Vector) (ImpactPoint :type Vector))
  (Game|SpawnActorfromClass "/Game/_Main/BluePrints/HUD/BulletDecal_BP.BulletDecal_BP_C" (Math|Transform|MakeTransform SpawnTransform (Math|Conversions|RotationFromXVector ImpactPoint) "0.025000,0.025000,0.025000") "Undefined" 0 0)
  (if (>= (Math|Random|RandomIntegerinRange 1 10) 7)
    (Game|SpawnActorfromClass "/Game/_Main/BluePrints/Weapons/TracerRounds_BP.TracerRounds_BP_C" (Math|Transform|MakeTransform Location (Transformation|GetWorldRotation (Variables|/Game/Bp_PlayerCharacter.Bp_PlayerCharacter_C|GetCameraComp (.AsBp%20Player%20Character (Utilities|Casting|CastToBp_PlayerCharacter (Game|GetPlayerCharacter 0))))) "0.100000,0.100000,0.100000") "Undefined" 0 0))
  (return))